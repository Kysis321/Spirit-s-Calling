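; A test platform that vanishes shortly after the player steps on it, then returns.
; When BP_Kyle_Test_PlayerCharachter enters the Box trigger, the Floor switches to a moving-water material, then hides and loses collision after a delay.
; Any end overlap immediately applies an emissive material, then restores visibility and collision after its own delay, without cancelling a pending disappearance.
; An unconnected cast to ThirdPersonCharacter never runs.
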(event OnComponentBeginOverlap(Box)
  (params (OverlappedComponent :type Primitive%20Component%20Object%20Reference) (OtherActor :type Actor%20Object%20Reference) (OtherComp :type Primitive%20Component%20Object%20Reference) (OtherBodyIndex :type Integer) (bFromSweep :type Boolean) (SweepResult :type Hit%20Result%20Structure%20%28by%20ref%29))
  (Utilities|Casting|CastToBP_Kyle_Test_PlayerCharachter OtherActor)
  (Rendering|Material|SetMaterial (Variables|Default|GetFloor) 0 "/Game/DreamscapeSeries/SharedResources/Materials/Terrain/M_Water_Moving.M_Water_Moving")
  (Utilities|FlowControl|Delay 3.0)
  (Rendering|SetVisibility (Variables|Default|GetFloor) false false)
  (Collision|SetCollisionEnabled (Variables|Default|GetFloor) "NoCollision"))

(event OnComponentEndOverlap(Box)
  (params (OverlappedComponent :type Primitive%20Component%20Object%20Reference) (OtherActor :type Actor%20Object%20Reference) (OtherComp :type Primitive%20Component%20Object%20Reference) (OtherBodyIndex :type Integer))
  (Rendering|Material|SetMaterial (Variables|Default|GetFloor) 0 "/Engine/ArtTools/RenderToTexture/Materials/Debug/M_Emissive_Color_0-0-127.M_Emissive_Color_0-0-127")
  (Utilities|FlowControl|Delay 3.0)
  (Rendering|SetVisibility (Variables|Default|GetFloor) true false)
  (Collision|SetCollisionEnabled (Variables|Default|GetFloor) "QueryAndPhysics"))

(fn ConstructionScript)