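; BP_MultigroundPoundBlock is a block actor that destroys itself once all five of its sigils are pressed.
; Five SetSigil events each latch a boolean and print a debug message.
; Tick polls the flags and, when all are true, prints a misleading "Not Set" message, then destroys the actor after a short Delay.
; The MultiStageGroundPoundDestruction event is an empty stub, and nothing here resets the flags.
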(event Custom|MultiStageGroundPoundDestruction)

(event Custom|SetSigilOne
  (Variables|Default|SetSigilOnePressed true)
  (Development|PrintString "SIGIL ONE SET"))

(event Custom|SetSigilFive
  (Variables|Default|SetSigilFivePressed true)
  (Development|PrintString "SIGIL Five SET"))

(event Custom|SetSigilTwo
  (Variables|Default|SetSigilTwoPressed true)
  (Development|PrintString "SIGIL TWO SET"))

(event Custom|SetSigilThree
  (Variables|Default|SetSigilThreePressed true)
  (Development|PrintString "SIGIL Three SET"))

(event Custom|SetSigilFour
  (Variables|Default|SetSigilFourPressed true)
  (Development|PrintString "SIGIL Four  SET"))

(event EventTick
  (params (DeltaSeconds :type Float%20%28single-precision%29))
  (if (and (Variables|Default|GetSigilOnePressed) (Variables|Default|GetSigilTwoPressed))
    (if (and (Variables|Default|GetSigilFourPressed) (Variables|Default|GetSigilThreePressed))
      (if (Variables|Default|GetSigilFivePressed)
        (Development|PrintString "Not Set")
        (Utilities|FlowControl|Delay 2.0)
        (Actor|DestroyActor)))))

(fn ConstructionScript)