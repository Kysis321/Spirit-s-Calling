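; Test orb pickup block that increments the Kyle test player character's OrbCount on overlap, shows the count, then destroys itself.
; The new count derives from the first player character found via GetAllActorsOfClass and is assigned to the overlapping one.
; Tick calls a colour-change event that creates a dynamic M_TestPickup material every frame and sets TestColour to black.
; Its orb-count threshold and colour lerp are unconnected, so the change is unconditional.
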(event OnComponentBeginOverlap(Zone)
  (params (OverlappedComponent :type Primitive%20Component%20Object%20Reference) (OtherActor :type Actor%20Object%20Reference) (OtherComp :type Primitive%20Component%20Object%20Reference) (OtherBodyIndex :type Integer) (bFromSweep :type Boolean) (SweepResult :type Hit%20Result%20Structure%20%28by%20ref%29))
  ;[1 1 1] Adding Orb Count to BP Kyle Test PlayerCharachter - Debug to show number collected
  (bind _asbp_kyle_test_player_charachter (Utilities|Casting|CastToBP_Kyle_Test_PlayerCharachter OtherActor))
  (bind _outactors (Actor|GetAllActorsOfClass "/Game/Spirits_Calling/0_Testing_Kyle/BP_Kyle_Test_PlayerCharachter.BP_Kyle_Test_PlayerCharachter_C"))
  (bind _result (Math|Float|IncrementFloat (Variables|/Game/Spirits_Calling/0_Testing_Kyle/BP_Kyle_Test_PlayerCharachter.BP_Kyle_Test_PlayerCharachter_C|GetOrbCount (Utilities|Array|Get(acopy) _outactors)))
    (:%20%20
      (Variables|/Game/Spirits_Calling/0_Testing_Kyle/BP_Kyle_Test_PlayerCharachter.BP_Kyle_Test_PlayerCharachter_C|SetOrbCount _asbp_kyle_test_player_charachter _result)
      (Default|ShowOrbCount _asbp_kyle_test_player_charachter)
      (Actor|DestroyActor))))

(event Custom|Colour%20change%20at10
  ;[1 1 1] Change Colour When Count is at 2
  (bind _asbp_kyle_test_player_charachter (Utilities|Casting|CastToBP_Kyle_Test_PlayerCharachter (Game|GetPlayerCharacter 0)))
  (bind _returnvalue (Rendering|Material|CreateDynamicMaterialInstance (Variables|Default|GetCube) 0 "/Game/Spirits_Calling/0_Testing_Kyle/M_TestPickup.M_TestPickup" "None" :!class /Script/Engine.PrimitiveComponent))
  (Rendering|Material|SetVectorParameterValue :self _returnvalue :ParameterName "TestColour" :!class /Script/Engine.MaterialInstanceDynamic))

(event EventTick
  (params (DeltaSeconds :type Float%20%28single-precision%29))
  ;[1 1 1] Check for update
  (CallFunction|ColourChangeat10))

(fn ConstructionScript)