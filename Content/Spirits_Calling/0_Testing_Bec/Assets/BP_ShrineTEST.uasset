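; Test shrine actor, apparently a prototype for clearing trash piles that share its ID when the player interacts.
; Its overlap events are effectively inert: begin is empty and end only casts to ThirdPersonCharacter.
; Disconnected logic holds input and prompt toggling plus a gated interaction that matches PlaceholderTrash by ID, calls CallShrine and spawns a light emitter.
; The matching loop takes no action, as the Destroy node is also unwired.
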(event OnComponentBeginOverlap(ShrineTrigger)
  (params (OverlappedComponent :type Primitive%20Component%20Object%20Reference) (OtherActor :type Actor%20Object%20Reference) (OtherComp :type Primitive%20Component%20Object%20Reference) (OtherBodyIndex :type Integer) (bFromSweep :type Boolean) (SweepResult :type Hit%20Result%20Structure%20%28by%20ref%29))
  ;[1 1 1] Enabling interaction with the E key when in the overlap (ShrineTrigger)
)

(event OnComponentEndOverlap(ShrineTrigger)
  (params (OverlappedComponent :type Primitive%20Component%20Object%20Reference) (OtherActor :type Actor%20Object%20Reference) (OtherComp :type Primitive%20Component%20Object%20Reference) (OtherBodyIndex :type Integer))
  ;[1 1 1] Enabling interaction with the E key when in the overlap (ShrineTrigger)
  (Utilities|Casting|CastToThirdPersonCharacter OtherActor))

(event Input|ActionEvents|InputActionInteract
  (params (Key :type Key%20Structure))
  ;[1 1 1] Enabling interaction with the E key when in the overlap (ShrineTrigger)
)

(fn ConstructionScript)