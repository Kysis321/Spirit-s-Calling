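; Game instance for Spirits Calling that holds the save data and relays level-load requests.
; On Init it loads the save slot into SaveGameData if one exists, otherwise it creates a new SaveGameObject in memory without writing it to disk.
; Event_LoadLevel, noted as called by UI_StartMenu, broadcasts the level name through the LoadLevel dispatcher for listeners such as PersistentLevel.
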(event Custom|Event_LoadLevel
  (params (Level%20Name :type Name))
  ;[1 1 1] When Event is called (By UI_StartMenu), caller passes input, event dispatcher sends input to anyone listening (PersistentLevel)
  (Default|CallLoadLevel Level%20Name false))

(event EventInit
  ;[1 0.06244 0.07239] Check to see if the save game file exits
  (bind _returnvalue (SaveGame|DoesSaveGameExist (Variables|Default|GetSaveSlotName)))
  (if _returnvalue
    ;[1 0.2959 0.166] If it does exist: we cast to it and load it & store it as a reference
    (bind _returnvalue_2 (SaveGame|LoadGamefromSlot (Variables|Default|GetSaveSlotName)))
    (bind _assave_game_object (Utilities|Casting|CastToSaveGameObject _returnvalue_2))
    (Variables|Default|SetSave%20Game%20Data _assave_game_object)
    (else
      ;[1 0.2747 0.205] If it doesnt exist. Create new save game data
      (bind _returnvalue_3 (SaveGame|CreateSaveGameObject "/Game/Spirits_Calling/Blueprints/Save_System(new)/SaveGameObject.SaveGameObject_C"))
      (Variables|Default|SetSave%20Game%20Data _returnvalue_3))))