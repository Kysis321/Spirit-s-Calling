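; GM_Credits, apparently the game mode for the credits in Spirits Calling, shows the ending cutscene UI and then the credits.
; On BeginPlay it adds UI_CutsceneEnd to the viewport at Z-order 1 and waits for the total duration of EndCutsceneFlipbook.
; It then adds UI_Credits at the default Z-order, beneath the cutscene widget, which this graph never removes.
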(event EventBeginPlay
  (bind _returnvalue (Game|GetPlayerController 0))
  (Utilities|FlowControl|Sequence
    (:then_0
      (bind _returnvalue_2 (UserInterface|CreateWidget "/Game/Spirits_Calling/Blueprints/Cutscenes/UI_CutsceneEnd.UI_CutsceneEnd_C" _returnvalue))
      (bind _output_get (Variables|Default|SetEndCutscene _returnvalue_2))
      (UserInterface|Viewport|AddtoViewport _output_get 1))
    (:then_1
      (Utilities|FlowControl|Delay (Class|PaperFlipbook|GetTotalDuration (Variables|Default|GetEndCutsceneFlipbook)))
      (bind _returnvalue_3 (UserInterface|CreateWidget "/Game/Spirits_Calling/Blueprints/UI_Blueprints/UI_Credits.UI_Credits_C" _returnvalue))
      (bind _output_get_2 (Variables|Default|SetCredits _returnvalue_3))
      (UserInterface|Viewport|AddtoViewport _output_get_2 0))))

(fn ConstructionScript)