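; Player controller for Spirits Calling that manages the pause menu, skill window closing, interaction prompts and a first-collectible dialogue.
; The pause input records keyboard or gamepad use in the game instance, then closes an open skill window or toggles the cached pause menu and game pause.
; Keyboard users get a mouse cursor, while gamepad users get delayed focus on Resume.
; Events create and remove prompt widgets and show the dialogue box after a delay.
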(event Custom|Show%20Prompt
  (params (Prompt :type Text))
  ;[1 1 1] Prompt System
  (bind _returnvalue (UserInterface|CreateWidget "/Game/Spirits_Calling/Blueprints/UI_Blueprints/UI_InteractPrompt.UI_InteractPrompt_C" (Game|GetPlayerController 0)))
  (bind _output_get (Variables|Default|SetPromptWidget _returnvalue))
  (UserInterface|Viewport|AddtoViewport _output_get 0)
  (Variables|/Game/Spirits_Calling/Blueprints/UI_Blueprints/UI_InteractPrompt.UI_InteractPrompt_C|SetPromptText _output_get Prompt))

(event Custom|Hide%20Prompt
  ;[1 1 1] Prompt System
  (Widget|RemovefromParent (stale Custom|Show%20Prompt _output_get)))

(event Custom|Close%20Skill%20Window
  (bind _returnvalue (Game|GetPlayerCharacter 0))
  (bind _returnvalue_2 (Game|GetPlayerController 0))
  ;[1 1 1] Pause Menu Toggle Functionality AND closing Skill window with Esc/P
  (Game|Player|SetViewTargetwithBlend _returnvalue 0.5 "VTBlend_Linear" 0.0 false)
  (Input|SetInputModeGameOnly _returnvalue_2)
  (Variables|/Script/Engine.PlayerController|SetbShowMouseCursor _returnvalue_2 false)
  (Rendering|SetActorHiddenInGame _returnvalue false)
  (Variables|Default|SetIsSkillWindowOpen false)
  (Variables|/Game/Spirits_Calling/Blueprints/BP_Stag.BP_Stag_C|SetIsWindowOpen (Variables|Default|GetBP_Stag) false))

(event Custom|Close%20Pause%20Menu
  (bind _returnvalue (Game|GetPlayerController 0))
  ;[1 1 1] Pause Menu Toggle Functionality AND closing Skill window with Esc/P
  (Game|SetGamePaused false)
  (Variables|/Script/Engine.PlayerController|SetbShowMouseCursor _returnvalue false)
  (Input|SetInputModeGameOnly _returnvalue)
  (Variables|Default|SetIsPauseMenuSet false))

(event Custom|FirstCollectibleDialogue
  ;[1 1 1] FirstCollectible Dialogue Box trigger
  (Utilities|FlowControl|Delay 3.0)
  (bind _returnvalue (UserInterface|CreateWidget "/Game/Spirits_Calling/Blueprints/UI_Blueprints/DialogueBox/UI_DialogueBox.UI_DialogueBox_C" (Game|GetPlayerController 0)))
  (bind _output_get (Variables|Default|SetUI_DialogueBox _returnvalue))
  (Variables|/Game/Spirits_Calling/Blueprints/UI_Blueprints/DialogueBox/UI_DialogueBox.UI_DialogueBox_C|SetDialogueRow _output_get "FirstCollectible")
  (UserInterface|Viewport|AddtoViewport _output_get 0))

(event EventBeginPlay
  ;[1 1 1] Pause Menu Toggle Functionality AND closing Skill window with Esc/P
  (bind _returnvalue (UserInterface|CreateWidget "/Game/Spirits_Calling/Blueprints/UI_Blueprints/UI_PauseMenu.UI_PauseMenu_C" (Game|GetPlayerController 0)))
  (Variables|Default|SetPauseMenu%20REF _returnvalue)
  (Variables|Default|SetIsPauseMenuSet true)
  (bind _asgi_spirits_calling (Utilities|Casting|CastToGI_SpiritsCalling (Game|GetGameInstance)))
  (Variables|Default|SetGI%20Spirits%20Calling _asgi_spirits_calling))

(event Input|ActionEvents|InputActionPauseGame
  (params (Key :type Key%20Structure :default "None"))
  (bind _returnvalue (Game|GetPlayerController 0))
  (bind _skillwindowui (Variables|Default|GetSkillWindowUI))
  ;[1 1 1] Pause Menu Toggle Functionality AND closing Skill window with Esc/P
  (:Pressed
    (Utilities|IsValid (Variables|Default|GetPauseMenu%20REF)
      (:Is%20Valid
        (bind _output_get (Variables|/Game/Spirits_Calling/Blueprints/UI_Blueprints/UI_PauseMenu.UI_PauseMenu_C|SetIsKeyboard (Variables|Default|GetPauseMenu%20REF) (Class|KismetInputLibrary|KeyIsKeyboardKey Key)))
        (bind _asgi_spirits_calling (Utilities|Casting|CastToGI_SpiritsCalling (Game|GetGameInstance)))
        (Variables|/Game/Spirits_Calling/Blueprints/GI_SpiritsCalling.GI_SpiritsCalling_C|SetIsKeyboard_GI _asgi_spirits_calling _output_get)
        (if (Variables|Default|GetIsSkillWindowOpen)
          (Utilities|IsValid _skillwindowui
            (:Is%20Valid
              (Default|CloseWindow _skillwindowui)))
          (else
            (Utilities|IsValid (Variables|Default|GetPauseMenu%20REF)
              (:Is%20Valid
                (if (Game|IsGamePaused)
                  (Development|PrintString "Close Menu" true true "(R=0.930735,G=0.256448,B=1.000000,A=1.000000)")
                  (Default|CloseWindow (Variables|Default|GetPauseMenu%20REF))
                  (else
                    (if (Variables|Default|GetIsPauseMenuSet)
                      _
                      (else
                        (bind _returnvalue_2 (UserInterface|CreateWidget "/Game/Spirits_Calling/Blueprints/UI_Blueprints/UI_PauseMenu.UI_PauseMenu_C" (Game|GetPlayerController 0)))
                        (bind _output_get_2 (Variables|Default|SetPauseMenu%20REF _returnvalue_2))))
                    (UserInterface|Viewport|AddtoViewport _output_get_2 0)
                    (Game|SetGamePaused true)
                    (if (Variables|/Game/Spirits_Calling/Blueprints/GI_SpiritsCalling.GI_SpiritsCalling_C|GetIsKeyboard_GI (Variables|Default|GetGI%20Spirits%20Calling))
                      (Variables|/Script/Engine.PlayerController|SetbShowMouseCursor _returnvalue true)
                      (Input|SetInputModeUIOnly _returnvalue (Variables|Default|GetPauseMenu%20REF) "LockInFullscreen")
                      (else
                        (Input|SetInputModeUIOnly _returnvalue (Variables|Default|GetPauseMenu%20REF) "LockInFullscreen")
                        (Utilities|FlowControl|Delay 0.2)
                        (Widget|SetKeyboardFocus (Variables|/Game/Spirits_Calling/Blueprints/UI_Blueprints/UI_PauseMenu.UI_PauseMenu_C|GetResume_UI (Variables|Default|GetPauseMenu%20REF)))))))))))))))

(fn ConstructionScript)