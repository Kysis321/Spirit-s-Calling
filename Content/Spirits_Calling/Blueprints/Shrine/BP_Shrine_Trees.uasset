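; BP_Shrine_Trees is the tree shrine that the player activates with Interact to clear its linked trash.
; Overlapping the trigger enables input, shows a prompt and opens a gate for the key press.
; Activation notifies the game mode, updates music, swaps material and reveals particles with a one-shot sound.
; It also fires a tree-shrine dispatcher and dissolves TrashTrees, destroying it after a short delay so the effect shows.
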(event OnComponentBeginOverlap(ShrineTrigger)
  (params (OverlappedComponent :type Primitive%20Component%20Object%20Reference) (OtherActor :type Actor%20Object%20Reference) (OtherComp :type Primitive%20Component%20Object%20Reference) (OtherBodyIndex :type Integer) (bFromSweep :type Boolean) (SweepResult :type Hit%20Result%20Structure%20%28by%20ref%29))
  (bind _trashtrees (Variables|Default|GetTrashTrees))
  ;[1 1 1] Enabling interaction with the E key when in the overlap (StagTrigger)
  (Utilities|Casting|CastToThirdPersonCharacter OtherActor)
  (if (Variables|Default|GetIsShrineOff)
    (Input|EnableInput (Game|GetPlayerController 0))
    ;[1 1 1] On Screen prompt will be displayed when in the overlap
    (|DoOnceMultiInput
      (:A%20Out
        (bind _aspcon_spirits_calling (Utilities|Casting|CastToPCon_SpiritsCalling (Game|GetPlayerController 0)))
        (Default|ShowPrompt _aspcon_spirits_calling (Variables|Default|GetPrompt))
        (Utilities|FlowControl|Gate false) ; enters at Open
      )
      (:Reset%20Out
        (Utilities|FlowControl|Gate false) ; enters at Close
      ))))

(event OnComponentEndOverlap(ShrineTrigger)
  (params (OverlappedComponent :type Primitive%20Component%20Object%20Reference) (OtherActor :type Actor%20Object%20Reference) (OtherComp :type Primitive%20Component%20Object%20Reference) (OtherBodyIndex :type Integer))
  (bind _trashtrees (Variables|Default|GetTrashTrees))
  ;[1 1 1] Enabling interaction with the E key when in the overlap (StagTrigger)
  (Utilities|Casting|CastToThirdPersonCharacter OtherActor)
  (Input|DisableInput (Game|GetPlayerController 0))
  ;[1 1 1] On Screen prompt will be displayed when in the overlap
  (bind _aspcon_spirits_calling (Utilities|Casting|CastToPCon_SpiritsCalling (Game|GetPlayerController 0)))
  (Default|HidePrompt _aspcon_spirits_calling)
  (|DoOnceMultiInput) ; enters at Reset In
)

(event Input|ActionEvents|InputActionInteract
  (params (Key :type Key%20Structure :default "None"))
  (bind _trashtrees (Variables|Default|GetTrashTrees))
  ;[1 1 1] Enabling interaction with the E key when in the overlap (StagTrigger)
  (:Pressed
    (Utilities|FlowControl|Gate false
      (:Exit
        (Utilities|FlowControl|Sequence
          (:then_0
            (bind _asgm_spirits_calling (Utilities|Casting|CastToGM_SpiritsCalling (Game|GetGameMode)))
            (if (Variables|Default|GetIsShrineOff)
              (Default|CollectedShrines _asgm_spirits_calling)
              (Variables|Default|SetIsShrineOff false)
              (Rendering|Material|SetMaterial (Variables|Default|GetShrine) 0 (Variables|Default|GetTriggeredMaterial))
              (Default|UpdateBGM _asgm_spirits_calling)))
          (:then_1
            (Default|CallTreesShrineDispatch)
            (Default|DissolveTrash _trashtrees) ; Call BP_TrashBog custom event
            ;[1 1 1] Gives time for dissolve material to show before being destroyed
            (Utilities|FlowControl|Delay 1.4)
            (Actor|DestroyActor _trashtrees))
          (:then_2
            ;[0 0.4012 1] This plays the audio once the shine has been activated
            (Utilities|FlowControl|DoOnce false
              (:Completed
                (Audio|PlaySoundatLocation "/Game/Spirits_Calling/Audio/Shrine/Shrine_Activate_Cue.Shrine_Activate_Cue" (Transformation|GetActorLocation) "0, 0, 0" 1.0 1.0 0.0 0 0 0))))
          (:then_3
            ;[0 1 0.545] Sets visability for particle system once the shrine is activated
            (Rendering|SetVisibility (Variables|Default|GetParticleSystem) true false)))))))

(fn ConstructionScript)