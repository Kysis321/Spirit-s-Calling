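; The stag is an interactable world actor that opens the skill purchase window when the player presses Interact nearby.
; Its StagTrigger overlap toggles input and a Gate for the third-person character.
; Interacting plays the stag's voice, blends the view to the stag, hides the player and, after a short delay, shows the UI_SkillWindow widget.
; It then flags the window open and links it to the character and three purchase buttons.
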(event OnComponentBeginOverlap(StagTrigger)
  (params (OverlappedComponent :type Primitive%20Component%20Object%20Reference) (OtherActor :type Actor%20Object%20Reference) (OtherComp :type Primitive%20Component%20Object%20Reference) (OtherBodyIndex :type Integer) (bFromSweep :type Boolean) (SweepResult :type Hit%20Result%20Structure%20%28by%20ref%29))
  (bind _returnvalue (Game|GetPlayerController 0))
  (bind _returnvalue_2 (Game|GetPlayerCharacter 0))
  ;[1 1 1] Enabling interaction with the E key when in the overlap (StagTrigger)
  (Utilities|Casting|CastToThirdPersonCharacter OtherActor)
  (Input|EnableInput (Game|GetPlayerController 0))
  (Utilities|FlowControl|Gate true) ; enters at Open
)

(event OnComponentEndOverlap(StagTrigger)
  (params (OverlappedComponent :type Primitive%20Component%20Object%20Reference) (OtherActor :type Actor%20Object%20Reference) (OtherComp :type Primitive%20Component%20Object%20Reference) (OtherBodyIndex :type Integer))
  (bind _returnvalue (Game|GetPlayerController 0))
  (bind _returnvalue_2 (Game|GetPlayerCharacter 0))
  ;[1 1 1] Enabling interaction with the E key when in the overlap (StagTrigger)
  (Utilities|Casting|CastToThirdPersonCharacter OtherActor)
  (Input|DisableInput (Game|GetPlayerController 0))
  (Utilities|FlowControl|Gate true) ; enters at Close
)

(event Input|ActionEvents|InputActionInteract
  (params (Key :type Key%20Structure :default "None"))
  (bind _returnvalue (Game|GetPlayerController 0))
  (bind _returnvalue_2 (Game|GetPlayerCharacter 0))
  ;[1 1 1] Enabling interaction with the E key when in the overlap (StagTrigger)
  (:Pressed
    (if (not (Variables|Default|GetIsWindowOpen))
      (Utilities|FlowControl|Gate true
        (:Exit
          ;[1 1 1] Changing camera, locking player character, hiding player character
          (Audio|PlaySoundatLocation "/Game/Spirits_Calling/Audio/NPC/Stag_Voice__audio_sample__Cue.Stag_Voice__audio_sample__Cue" (Transformation|GetActorLocation) "0, 0, 0" 1.0 1.0 0.0 0 0 0)
          (Game|Player|SetViewTargetwithBlend _returnvalue self 0.5 "VTBlend_Linear" 0.0 false)
          (bind _returnvalue_3 (UserInterface|CreateWidget "/Game/Spirits_Calling/Blueprints/UI_Blueprints/UI_SkillWindow.UI_SkillWindow_C" _returnvalue))
          (Variables|Default|SetSkillWindow _returnvalue_3)
          (Variables|/Script/Engine.PlayerController|SetbShowMouseCursor _returnvalue true)
          (Rendering|SetActorHiddenInGame _returnvalue_2 true)
          (Utilities|FlowControl|Delay 0.6)
          (UserInterface|Viewport|AddtoViewport (Variables|Default|GetSkillWindow) 0)
          (Input|SetInputModeGameandUI (Game|GetPlayerController 0) (Variables|Default|GetSkillWindow) "DoNotLock" false)
          (bind _asthird_person_character (Utilities|Casting|CastToThirdPersonCharacter _returnvalue_2))
          (Variables|/Game/Spirits_Calling/Blueprints/ThirdPersonCharacter.ThirdPersonCharacter_C|SetIsSkillWindowOpen _asthird_person_character true)
          (Variables|Default|SetIsWindowOpen true)
          (Variables|/Game/Spirits_Calling/Blueprints/ThirdPersonCharacter.ThirdPersonCharacter_C|SetSkillMenuUI _asthird_person_character (Variables|Default|GetSkillWindow))
          (Variables|/Game/Spirits_Calling/Blueprints/UI_Blueprints/UI_SkillPurchaseButton.UI_SkillPurchaseButton_C|SetMySkillWindowUI (Variables|/Game/Spirits_Calling/Blueprints/UI_Blueprints/UI_SkillWindow.UI_SkillWindow_C|GetSkillPurchaseButton_DJ (Variables|Default|GetSkillWindow)) (Variables|Default|GetSkillWindow))
          (Variables|/Game/Spirits_Calling/Blueprints/UI_Blueprints/UI_SkillPurchaseButton.UI_SkillPurchaseButton_C|SetMySkillWindowUI (Variables|/Game/Spirits_Calling/Blueprints/UI_Blueprints/UI_SkillWindow.UI_SkillWindow_C|GetSkillPurchaseButton_D (Variables|Default|GetSkillWindow)) (Variables|Default|GetSkillWindow))
          (Variables|/Game/Spirits_Calling/Blueprints/UI_Blueprints/UI_SkillPurchaseButton.UI_SkillPurchaseButton_C|SetMySkillWindowUI (Variables|/Game/Spirits_Calling/Blueprints/UI_Blueprints/UI_SkillWindow.UI_SkillWindow_C|GetSkillPurchaseButton_GP (Variables|Default|GetSkillWindow)) (Variables|Default|GetSkillWindow)))))))

(fn ConstructionScript)