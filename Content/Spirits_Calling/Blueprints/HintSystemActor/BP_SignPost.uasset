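; Signpost actor that shows a hint to the player on pressing Interact inside its trigger.
; Overlap enables input, shows a prompt through PCon_SpiritsCalling and opens a gate for the Interact press.
; Interacting hides the prompt, blends the view to the signpost and, after a short delay, displays a UI_HintSystem widget for its HintRowName.
; Leaving disables input, hides the prompt, and restores the character view and ends any open hint.
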(event OnComponentBeginOverlap(HintTrigger)
  (params (OverlappedComponent :type Primitive%20Component%20Object%20Reference) (OtherActor :type Actor%20Object%20Reference) (OtherComp :type Primitive%20Component%20Object%20Reference) (OtherBodyIndex :type Integer) (bFromSweep :type Boolean) (SweepResult :type Hit%20Result%20Structure%20%28by%20ref%29))
  (bind _returnvalue (Game|GetPlayerController 0))
  ;[1 1 1] Enabling interaction with the E key when in the overlap (StagTrigger)
  (Utilities|Casting|CastToThirdPersonCharacter OtherActor)
  (Input|EnableInput (Game|GetPlayerController 0))
  ;[1 1 1] On Screen prompt will be displayed when in the overlap
  (|DoOnceMultiInput
    (:A%20Out
      (bind _aspcon_spirits_calling (Utilities|Casting|CastToPCon_SpiritsCalling (Game|GetPlayerController 0)))
      (Default|ShowPrompt _aspcon_spirits_calling (Variables|Default|GetPrompt))
      ;[1 1 1] When interact key pressed, remove prompt from viewport, change camera, create hint system and set to viewport
      (Utilities|FlowControl|Gate false) ; enters at Open
    )
    (:Reset%20Out
      (Utilities|FlowControl|Gate false) ; enters at Close
    )))

(event OnComponentEndOverlap(HintTrigger)
  (params (OverlappedComponent :type Primitive%20Component%20Object%20Reference) (OtherActor :type Actor%20Object%20Reference) (OtherComp :type Primitive%20Component%20Object%20Reference) (OtherBodyIndex :type Integer))
  (bind _returnvalue (Game|GetPlayerController 0))
  ;[1 1 1] Enabling interaction with the E key when in the overlap (StagTrigger)
  (Utilities|Casting|CastToThirdPersonCharacter OtherActor)
  (Utilities|FlowControl|Sequence
    (:then_0
      (Input|DisableInput (Game|GetPlayerController 0))
      ;[1 1 1] On Screen prompt will be displayed when in the overlap
      (bind _aspcon_spirits_calling (Utilities|Casting|CastToPCon_SpiritsCalling (Game|GetPlayerController 0)))
      (Default|HidePrompt _aspcon_spirits_calling)
      (|DoOnceMultiInput) ; enters at Reset In
    )
    (:then_1
      ;[1 1 1] If player moves out of overlap, reset camera and remove widget
      (if (Variables|Default|GetIsHintOpen)
        (Game|Player|SetViewTargetwithBlend (Game|GetPlayerController 0) (Game|GetPlayerCharacter 0) 0.5 "VTBlend_Linear" 0.0 false)
        (Variables|Default|SetIsHintOpen false)
        (Default|EndOverlap (Variables|Default|GetUI_HintSystem))))))

(event Input|ActionEvents|InputActionInteract
  (params (Key :type Key%20Structure :default "None"))
  (bind _returnvalue (Game|GetPlayerController 0))
  ;[1 1 1] Enabling interaction with the E key when in the overlap (StagTrigger)
  (:Pressed
    ;[1 1 1] When interact key pressed, remove prompt from viewport, change camera, create hint system and set to viewport
    (Utilities|FlowControl|Gate false
      (:Exit
        (bind _aspcon_spirits_calling (Utilities|Casting|CastToPCon_SpiritsCalling (Game|GetPlayerController 0)))
        (Default|HidePrompt _aspcon_spirits_calling)
        (Game|Player|SetViewTargetwithBlend _returnvalue self 0.5 "VTBlend_Linear" 0.0 false)
        (bind _returnvalue_2 (UserInterface|CreateWidget "/Game/Spirits_Calling/Blueprints/UI_Blueprints/HintSystem/UI_HintSystem.UI_HintSystem_C" _returnvalue))
        (bind _output_get (Variables|Default|SetUI_HintSystem _returnvalue_2))
        (Utilities|FlowControl|Delay 0.6)
        (Variables|/Game/Spirits_Calling/Blueprints/UI_Blueprints/HintSystem/UI_HintSystem.UI_HintSystem_C|SetHintRowName _output_get (Variables|Default|GetHintRowName))
        (UserInterface|Viewport|AddtoViewport _output_get 0)
        (Variables|Default|SetIsHintOpen true)))))

(fn ConstructionScript)