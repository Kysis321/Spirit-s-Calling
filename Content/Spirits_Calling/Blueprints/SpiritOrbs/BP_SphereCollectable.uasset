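; Spirit orb pickup that reports to GM_SpiritsCalling when the third-person character overlaps it.
; Collection disables collision and plays a sound while the Attraction timeline lerps the orb mesh from its current location toward the moving character, then destroys the actor.
; A separate sound sphere spawns an ambience cue on character entry and fades out the AmbientSound component on exit, rather than the spawned sound.
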(event OnComponentBeginOverlap(SpiritOrb_Collision)
  (params (OverlappedComponent :type Primitive%20Component%20Object%20Reference) (OtherActor :type Actor%20Object%20Reference) (OtherComp :type Primitive%20Component%20Object%20Reference) (OtherBodyIndex :type Integer) (bFromSweep :type Boolean) (SweepResult :type Hit%20Result%20Structure%20%28by%20ref%29))
  ;[1 1 1] When the player passes over the spirit orb
  (bind _asthird_person_character (Utilities|Casting|CastToThirdPersonCharacter OtherActor))
  (bind _asgm_spirits_calling (Utilities|Casting|CastToGM_SpiritsCalling (Game|GetGameMode)))
  ;[1 1 1] As 0.5 seconds pass the gem will move from a to b. B being the character location
  (Default|CollectedOrbs _asgm_spirits_calling)
  (Collision|SetCollisionEnabled (Variables|Default|GetSpiritOrb_Collision) "NoCollision")
  ;[1 0.3353 0.9757] Sound spawner for collectable. (activates only when the player collects the spirit orb)
  (Utilities|FlowControl|Sequence
    (:then_0
      (Audio|SpawnSoundatLocation "/Game/Spirits_Calling/Audio/Environment/Spirit_Orb_Collectible_Cue.Spirit_Orb_Collectible_Cue" (Transformation|GetActorLocation) "0, 0, 0" 1.0 1.0 0.0 0 0))
    (:then_1
      (bind _distance_normalised_ (Timeline|Attraction Play)
        (:Update
          (Transformation|SetWorldLocation (Variables|Default|GetSpiritOrb) (Math|Vector|Lerp(Vector) (Transformation|GetWorldLocation (Variables|Default|GetSpiritOrb)) (Transformation|GetActorLocation _asthird_person_character) _distance_normalised_) false false))
        (:Finished
          ;[1 1 1] Once the animation is complete Destroy the spirit orb
          (Actor|DestroyActor))))))

(event OnComponentBeginOverlap(SoundColSphere)
  (params (OverlappedComponent :type Primitive%20Component%20Object%20Reference) (OtherActor :type Actor%20Object%20Reference) (OtherComp :type Primitive%20Component%20Object%20Reference) (OtherBodyIndex :type Integer) (bFromSweep :type Boolean) (SweepResult :type Hit%20Result%20Structure%20%28by%20ref%29))
  ;[1 0.2486 0.8262] Audio for ambience. Fades in and out based on collision
  (Utilities|Casting|CastToThirdPersonCharacter OtherActor)
  (Audio|SpawnSoundatLocation "/Game/Spirits_Calling/Audio/Environment/Orb_Ambience_Cue.Orb_Ambience_Cue" (Transformation|GetActorLocation) "0, 0, 0" 1.0 1.0 0.0 0 0))

(event OnComponentEndOverlap(SoundColSphere)
  (params (OverlappedComponent :type Primitive%20Component%20Object%20Reference) (OtherActor :type Actor%20Object%20Reference) (OtherComp :type Primitive%20Component%20Object%20Reference) (OtherBodyIndex :type Integer))
  ;[1 0.2486 0.8262] Audio for ambience. Fades in and out based on collision
  (Utilities|Casting|CastToThirdPersonCharacter OtherActor)
  (Audio|Components|Audio|FadeOut (Variables|Default|GetAmbient%20sound) 1.0 0.0 "Linear" :!class /Script/Engine.AudioComponent))

(event EventBeginPlay)

(event Collision|EventActorBeginOverlap
  (params (OtherActor :type Actor%20Object%20Reference)))

(fn ConstructionScript)