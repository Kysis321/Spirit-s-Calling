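; Collectable spirit orb that the player picks up by passing over it.
; On overlap with the ThirdPersonCharacter, it reports the pickup to GM_SpiritsCalling through CollectedOrbs and disables its collision.
; An Attraction timeline then lerps the orb from its current location toward the character's live position each update, and destroys the actor when finished.
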(event OnComponentBeginOverlap(SpiritOrb_Collision)
  (params (OverlappedComponent :type Primitive%20Component%20Object%20Reference) (OtherActor :type Actor%20Object%20Reference) (OtherComp :type Primitive%20Component%20Object%20Reference) (OtherBodyIndex :type Integer) (bFromSweep :type Boolean) (SweepResult :type Hit%20Result%20Structure%20%28by%20ref%29))
  ;[1 1 1] When the player passes over the spirit orb
  (bind _asthird_person_character (Utilities|Casting|CastToThirdPersonCharacter OtherActor))
  (bind _asgm_spirits_calling (Utilities|Casting|CastToGM_SpiritsCalling (Game|GetGameMode)))
  ;[1 1 1] As 0.5 seconds pass the gem will move from a to b. B being the character location
  (Default|CollectedOrbs _asgm_spirits_calling)
  (Collision|SetCollisionEnabled (Variables|Default|GetSpiritOrb_Collision) "NoCollision")
  (bind _distance_normalised_ (Timeline|Attraction Play)
    (:Update
      (Transformation|SetWorldLocation (Variables|Default|GetSpiritOrb) (Math|Vector|Lerp(Vector) (Transformation|GetWorldLocation (Variables|Default|GetSpiritOrb)) (Transformation|GetActorLocation _asthird_person_character) _distance_normalised_) false false))
    (:Finished
      ;[1 1 1] Once the animation is complete Destroy the spirit orb
      (Actor|DestroyActor))))

(event EventBeginPlay)

(event Collision|EventActorBeginOverlap
  (params (OtherActor :type Actor%20Object%20Reference)))

(event EventTick
  (params (DeltaSeconds :type Float%20%28single-precision%29)))

(fn ConstructionScript)