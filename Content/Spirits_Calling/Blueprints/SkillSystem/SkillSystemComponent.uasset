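; Skill system component that records which skills, such as a ground pound, have been unlocked.
; AddSkill stores each skill row name in the SkillUnlocks map with a count of 1, incrementing it on repeat additions and always returning true.
; QuerySkill reports whether a row name exists in that map, ignoring its count.
; The event graph holds only unused BeginPlay and Tick stubs.
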(event EventBeginPlay)

(event EventTick
  (params (DeltaSeconds :type Float%20%28single-precision%29)))

(fn AddSkill
  (params (row_name :type String))
  (bind _skillunlocks (Variables|Default|GetSkillUnlocks))
  (bind (_value _returnvalue) (Utilities|Map|Find _skillunlocks row_name))
  ;[0.9965 1 0.4729] adding a new skill
  (if _returnvalue
    (Utilities|Map|Add (Variables|Default|GetSkillUnlocks) row_name (+ _value 1))
    (return true)
    (else
      (Utilities|Map|Add (Variables|Default|GetSkillUnlocks) row_name 1)
      (return true))))

(fn QuerySkill
  (params (RowName :type String))
  ;[1 0.6562 0.6562] Checking if we have a particular move e.g ground pound
  (if (.ReturnValue (Utilities|Map|Find (Variables|Default|GetSkillUnlocks) RowName))
    (return true)
    (else
      (return false))))