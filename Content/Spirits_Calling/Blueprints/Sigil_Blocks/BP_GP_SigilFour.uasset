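; Ground-pound sigil block, the fourth sigil, that registers a press when the player character slams onto it.
; When the Detect volume is entered, a DoOnce gate, reset on exit, checks IsGroundPound at that moment and calls SigilFourPresed on the Target reference.
; A second, never-reset DoOnce plays the switch sound at the block only on the first successful press, alongside debug prints.
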(event OnComponentBeginOverlap(detect)
  (params (OverlappedComponent :type Primitive%20Component%20Object%20Reference) (OtherActor :type Actor%20Object%20Reference) (OtherComp :type Primitive%20Component%20Object%20Reference) (OtherBodyIndex :type Integer) (bFromSweep :type Boolean) (SweepResult :type Hit%20Result%20Structure%20%28by%20ref%29))
  (bind _asthird_person_character (Utilities|Casting|CastToThirdPersonCharacter OtherActor))
  (Utilities|FlowControl|DoOnce false
    (:Completed
      (if (Variables|/Game/Spirits_Calling/Blueprints/ThirdPersonCharacter.ThirdPersonCharacter_C|Getis_GroundPound _asthird_person_character)
        (Development|PrintString "sigil pressed ")
        (Default|SigilFourPresed (Variables|Default|GetTarget))
        ;[1 1 1] audio for sigil
        (Utilities|FlowControl|DoOnce false
          (:Completed
            (Audio|PlaySoundatLocation "/Game/Spirits_Calling/Audio/Environment/Switch__audio_sample__Cue.Switch__audio_sample__Cue" (Transformation|GetActorLocation) "0, 0, 0" 1.0 1.0 0.0 0 0 0)
            (Development|PrintString "sigilfourset")))))))

(event OnComponentEndOverlap(detect)
  (params (OverlappedComponent :type Primitive%20Component%20Object%20Reference) (OtherActor :type Actor%20Object%20Reference) (OtherComp :type Primitive%20Component%20Object%20Reference) (OtherBodyIndex :type Integer))
  (Utilities|Casting|CastToThirdPersonCharacter OtherActor)
  (Utilities|FlowControl|DoOnce false) ; enters at Reset
)

(fn ConstructionScript)