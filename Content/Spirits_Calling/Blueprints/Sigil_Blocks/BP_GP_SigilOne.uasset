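; BP_GP_SigilOne is a sigil trigger that the player activates by ground pounding it, feeding a multi-ground-pound block.
; When the player character begins overlapping Detect during a ground pound, it marks itself pushed and sets SigilOnePressed on the referenced Multiblock.
; The pound state is checked only on overlap entry, through a DoOnce that resets when the player leaves.
; Debug prints report success or failure.
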(event OnComponentBeginOverlap(detect)
  (params (OverlappedComponent :type Primitive%20Component%20Object%20Reference) (OtherActor :type Actor%20Object%20Reference) (OtherComp :type Primitive%20Component%20Object%20Reference) (OtherBodyIndex :type Integer) (bFromSweep :type Boolean) (SweepResult :type Hit%20Result%20Structure%20%28by%20ref%29))
  (bind _asbp_kyle_test_player_charachter (Utilities|Casting|CastToBP_Kyle_Test_PlayerCharachter OtherActor))
  (Utilities|FlowControl|DoOnce false
    (:Completed
      (if (Variables|/Game/Spirits_Calling/0_Testing_Kyle/BP_Kyle_Test_PlayerCharachter.BP_Kyle_Test_PlayerCharachter_C|Getis_GroundPound _asbp_kyle_test_player_charachter)
        (Variables|Default|SetisSigilOnePushed true)
        (bind _asbp_multiground_pound_block (Utilities|Casting|CastToBP_MultigroundPoundBlock (Variables|Default|GetMultiblock))
          (:then
            (Variables|/Game/Spirits_Calling/0_Testing_Kyle/GroundPounds_Assets/BP_MultigroundPoundBlock.BP_MultigroundPoundBlock_C|SetSigilOnePressed _asbp_multiground_pound_block true)
            (Development|PrintString "sigilOneset"))
          (:CastFailed
            (Development|PrintString "Fail")))
        (else
          (Development|PrintString "Not Ground Pound"))))))

(event OnComponentEndOverlap(detect)
  (params (OverlappedComponent :type Primitive%20Component%20Object%20Reference) (OtherActor :type Actor%20Object%20Reference) (OtherComp :type Primitive%20Component%20Object%20Reference) (OtherBodyIndex :type Integer))
  (Utilities|Casting|CastToBP_Kyle_Test_PlayerCharachter OtherActor)
  (Utilities|FlowControl|DoOnce false) ; enters at Reset
)

(fn ConstructionScript)