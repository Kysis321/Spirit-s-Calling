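; BP_TrashBog is a construction-script scatter actor that places random static meshes around itself, apparently as trash set dressing.
; It clamps the mesh count, then adds components with meshes picked randomly from MeshArray and optional random yaw.
; Offsets are flat and clamped to Radius, but only positive in X and Y, covering one quadrant.
; Scale always equals MinimumScale, since both random bounds use it.
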(fn ConstructionScript
  (bind _radius (Variables|Default|GetRadius))
  (bind _minimum_scale (Variables|Default|GetMinimum%20Scale))
  (bind _minimum_scale_2 (Variables|Default|GetMinimum%20Scale))
  (bind _mesharray (Variables|Default|GetMeshArray))
  (bind (_x _y _z) (Math|Vector|BreakVector _minimum_scale))
  (bind (_x_2 _y_2 _z_2) (Math|Vector|BreakVector _minimum_scale_2))
  (bind _returnvalue (* _radius 0.0))
  (Variables|Default|SetNumberofMeshes (Math|Integer|Clamp(Integer) (Variables|Default|GetNumberofMeshes) 0 5))
  (for _index (range 0 (Variables|Default|GetNumberofMeshes))
    (bind _returnvalue_2 (AddComponent|AddStaticMeshComponent false (Math|Transform|MakeTransform (Math|Vector|ClampVectorSize (Math|Vector|MakeVector (Math|Random|RandomFloatinRange _returnvalue _radius) (Math|Random|RandomFloatinRange _returnvalue _radius) 0.0) 0.0 (Variables|Default|GetRadius)) (Math|Rotator|SelectRotator (Math|Rotator|MakeRotator 0.0 0.0 (Math|Random|RandomFloatinRange 0.0 1e+02)) "0, 0, 0" (Variables|Default|GetRandomYawRotation)) (Math|Vector|MakeVector (Math|Random|RandomFloatinRange _x_2 _x) (Math|Random|RandomFloatinRange _y_2 _y) (Math|Random|RandomFloatinRange _z_2 _z)))))
    (Components|StaticMesh|SetStaticMesh _returnvalue_2 (Utilities|Array|Get(acopy) _mesharray (Math|Random|RandomIntegerinRange 0 (Utilities|Array|LastIndex _mesharray))))))