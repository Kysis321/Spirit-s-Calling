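; Trash mountain top actor that builds a randomized pile of trash and can switch it to a dissolve material.
; The construction script adds child actor components using random picks from ActorArray, with randomized placement within Radius.
; BeginPlay spawns and attaches bottle and coffee trash, then creates a dynamic M_Dissolve_2 instance.
; DissolveTrash applies that instance to material slot 0 on static meshes of every IDissolve-implementing BP_TrashMountainTop in the level.
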(event Custom|DissolveTrash
  ;[1 1 1] Change material of the trash bog
  (bind _outactors (Actor|GetAllActorsOfClass "BP_TrashMountainTop_C"))
  (for _array_element _outactors
    (if (Utilities|DoesObjectImplementInterface _array_element "/Game/Spirits_Calling/0_Testing_Alex/DissolveFX/IDissolve.IDissolve_C")
      (for _array_element_2 (Actor|GetComponentsByClass _array_element "/Script/Engine.StaticMeshComponent")
        (for _index (range 0 (- (Rendering|Material|GetNumMaterials _array_element_2) 1))
          (Rendering|Material|SetMaterial _array_element_2 0 (Variables|Default|GetDissolveMaterial)))))))

(event EventBeginPlay
  (bind _ref_to_self (Variables|Default|GetRef%20to%20Self))
  (Utilities|FlowControl|Sequence
    (:then_0
      (for _index (range 0 (Variables|Default|GetNo%20of%20Bottle))
        (bind _returnvalue (Game|SpawnActorfromClass "/Game/Spirits_Calling/Blueprints/Trash/BP_BottleTrashGravity.BP_BottleTrashGravity_C" (Math|Conversions|ToTransform(Vector) (Transformation|GetWorldLocation (Variables|Default|GetDefaultSceneRoot))) "Undefined" 0 0))
        (Transformation|AttachActorToActor _returnvalue _ref_to_self "None" "KeepWorld" "KeepWorld" "KeepWorld" true)))
    (:then_1
      (for _index_2 (range 0 (Variables|Default|GetNo%20of%20Coffee))
        (bind _returnvalue_2 (Game|SpawnActorfromClass "/Game/Spirits_Calling/Blueprints/Trash/BP_CoffeeTrash.BP_CoffeeTrash_C" (Math|Conversions|ToTransform(Vector) (Transformation|GetWorldLocation (Variables|Default|GetDefaultSceneRoot))) "Undefined" 0 0))
        (Transformation|AttachActorToActor _returnvalue_2 _ref_to_self "None" "KeepWorld" "KeepWorld" "KeepWorld" true)))
    (:then_2
      ;[1 1 1] Create dissolve material instance
      (bind _returnvalue_3 (Rendering|Material|CreateDynamicMaterialInstance "/Game/Spirits_Calling/0_Testing_Alex/DissolveFX/FX2/M_Dissolve_2.M_Dissolve_2" "None" "None" :!class /Script/Engine.KismetMaterialLibrary))
      (Variables|Default|SetDissolveMaterial _returnvalue_3))))

(fn ConstructionScript
  (bind _returnvalue (Math|Random|RandomFloatinRange 0.0 75.0))
  (bind _radius (Variables|Default|GetRadius))
  (bind _minimum_scale (Variables|Default|GetMinimum%20Scale))
  (bind _minimum_scale_2 (Variables|Default|GetMinimum%20Scale))
  (bind _actorarray (Variables|Default|GetActorArray))
  (bind (_x _y _z) (Math|Vector|BreakVector _minimum_scale))
  (bind (_x_2 _y_2 _z_2) (Math|Vector|BreakVector _minimum_scale_2))
  (bind _returnvalue_2 (* _radius 0.0))
  (Variables|Default|SetNumberofMeshes (Math|Integer|Clamp(Integer) (Variables|Default|GetNumberofMeshes) 0 5))
  (for _index (range 0 (Variables|Default|GetNumberofMeshes))
    (AddComponent|AddChildActorComponent (Utilities|Array|Get(acopy) _actorarray (Math|Random|RandomIntegerinRange 0 (Utilities|Array|LastIndex _actorarray))) false (Math|Transform|MakeTransform (Math|Vector|ClampVectorSize (Math|Vector|MakeVector (Math|Random|RandomFloatinRange _returnvalue_2 _radius) (Math|Random|RandomFloatinRange _returnvalue_2 _radius) 0.0) 0.0 (Variables|Default|GetRadius)) (Math|Rotator|SelectRotator (Math|Rotator|MakeRotator _returnvalue _returnvalue _returnvalue) "0, 0, 0" (Variables|Default|GetRandomYawRotation)) (Math|Vector|MakeVector (Math|Random|RandomFloatinRange _x_2 _x) (Math|Random|RandomFloatinRange _y_2 _y) (Math|Random|RandomFloatinRange _z_2 _z))))))