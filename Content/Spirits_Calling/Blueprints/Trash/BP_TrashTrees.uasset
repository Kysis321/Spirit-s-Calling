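; BP_TrashTrees is a trash actor that scatters random meshes around itself and can be dissolved away.
; The construction script spawns a clamped number of meshes from MeshArray at random offsets within Radius, with optional random rotation.
; BeginPlay creates a dynamic dissolve material.
; DissolveTrash applies it to material slot 0 on meshes of every BP_TrashTrees implementing ITrashDissolve_Trees, then destroys only itself after a short delay.
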(event Custom|DissolveTrash
  ;[1 1 1] Change material of the trash bog
  (bind _outactors (Actor|GetAllActorsOfClass "BP_TrashTrees_C"))
  (for _array_element _outactors
    (if (Utilities|DoesObjectImplementInterface _array_element "/Game/Spirits_Calling/Blueprints/Trash/ITrashDissolve_Trees.ITrashDissolve_Trees_C")
      (for _array_element_2 (Actor|GetComponentsByClass _array_element "/Script/Engine.StaticMeshComponent")
        (for _index (range 0 (- (Rendering|Material|GetNumMaterials _array_element_2) 1))
          (Rendering|Material|SetMaterial _array_element_2 0 (Variables|Default|GetDissolveMaterial))))))
  (Utilities|FlowControl|Delay 1.4)
  (Actor|DestroyActor))

(event EventBeginPlay
  ;[1 1 1] Create dissolve material instance
  (bind _returnvalue (Rendering|Material|CreateDynamicMaterialInstance "/Game/Spirits_Calling/0_Testing_Alex/DissolveFX/FX2/M_Dissolve_2.M_Dissolve_2" "None" "None" :!class /Script/Engine.KismetMaterialLibrary))
  (Variables|Default|SetDissolveMaterial _returnvalue))

(fn ConstructionScript
  (bind _returnvalue (Math|Random|RandomFloatinRange 0.0 1e+02))
  (bind _radius (Variables|Default|GetRadius))
  (bind _minimum_scale (Variables|Default|GetMinimum%20Scale))
  (bind _minimum_scale_2 (Variables|Default|GetMinimum%20Scale))
  (bind _mesharray (Variables|Default|GetMeshArray))
  (bind (_x _y _z) (Math|Vector|BreakVector _minimum_scale))
  (bind (_x_2 _y_2 _z_2) (Math|Vector|BreakVector _minimum_scale_2))
  (bind _returnvalue_2 (* _radius 0.0))
  (Variables|Default|SetNumberofMeshes (Math|Integer|Clamp(Integer) (Variables|Default|GetNumberofMeshes) 0 5))
  (for _index (range 0 (Variables|Default|GetNumberofMeshes))
    (bind _returnvalue_3 (AddComponent|AddStaticMeshComponent false (Math|Transform|MakeTransform (Math|Vector|ClampVectorSize (Math|Vector|MakeVector (Math|Random|RandomFloatinRange _returnvalue_2 _radius) (Math|Random|RandomFloatinRange _returnvalue_2 _radius) 0.0) 0.0 (Variables|Default|GetRadius)) (Math|Rotator|SelectRotator (Math|Rotator|MakeRotator _returnvalue _returnvalue _returnvalue) "0, 0, 0" (Variables|Default|GetRandomYawRotation)) (Math|Vector|MakeVector (Math|Random|RandomFloatinRange _x_2 _x) (Math|Random|RandomFloatinRange _y_2 _y) (Math|Random|RandomFloatinRange _z_2 _z)))))
    (Components|StaticMesh|SetStaticMesh _returnvalue_3 (Utilities|Array|Get(acopy) _mesharray (Math|Random|RandomIntegerinRange 0 (Utilities|Array|LastIndex _mesharray))))))