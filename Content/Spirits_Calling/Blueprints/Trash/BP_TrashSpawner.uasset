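; Trash pile spawner that fills its location with assorted litter actors and can dissolve them away.
; BeginPlay spawns configurable counts of bottles, coffee, milk, cans and bags at the root into MeshArray, then creates one shared dynamic dissolve material.
; DissolveTrash applies that material to slot 0 of each mesh, waits briefly, then hides and destroys the actors.
; The construction script's random mesh scattering is disconnected, leaving an empty loop.
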(event Custom|DissolveTrash
  (bind _mesharray (Variables|Default|GetMeshArray))
  ;[1 1 1] Change material of the trash bog
  (for _array_element _mesharray
    (for _index (range 0 (- (Rendering|Material|GetNumMaterials (Actor|GetComponentbyClass _array_element "/Script/Engine.StaticMeshComponent")) 1))
      (Rendering|Material|SetMaterial (Actor|GetComponentbyClass _array_element "/Script/Engine.StaticMeshComponent") 0 (Variables|Default|GetDissolveMaterial))))
  (Utilities|FlowControl|Delay 0.9)
  (bind _arrayelement (Utilities|Array|ReverseforEachLoop _mesharray)
    (:LoopBody
      (Rendering|SetActorHiddenInGame _arrayelement true)
      (Actor|DestroyActor _arrayelement))))

(event EventBeginPlay
  (bind _mesharray (Variables|Default|GetMeshArray))
  (bind _mesharray_2 (Variables|Default|GetMeshArray))
  (bind _mesharray_3 (Variables|Default|GetMeshArray))
  (Utilities|FlowControl|Sequence
    (:then_0
      (for _index (range 0 (Variables|Default|GetNo%20of%20Bottle))
        (bind _returnvalue (Game|SpawnActorfromClass "/Game/Spirits_Calling/Blueprints/Trash/BP_BottleTrashGravity.BP_BottleTrashGravity_C" (Math|Conversions|ToTransform(Vector) (Transformation|GetWorldLocation (Variables|Default|GetDefaultSceneRoot))) "Undefined" 0 0))
        (Utilities|Array|Add _mesharray_2 _returnvalue)))
    (:then_1
      (for _index_2 (range 0 (Variables|Default|GetNo%20of%20Coffee))
        (bind _returnvalue_2 (Game|SpawnActorfromClass "/Game/Spirits_Calling/Blueprints/Trash/BP_CoffeeTrash.BP_CoffeeTrash_C" (Math|Conversions|ToTransform(Vector) (Transformation|GetWorldLocation (Variables|Default|GetDefaultSceneRoot))) "Undefined" 0 0))
        (Utilities|Array|Add _mesharray_2 _returnvalue_2)))
    (:then_2
      (for _index_3 (range 0 (Variables|Default|GetNo%20of%20BotCrunched))
        (bind _returnvalue_3 (Game|SpawnActorfromClass "/Game/Spirits_Calling/Blueprints/Trash/BP_BotteCrunched.BP_BotteCrunched_C" (Math|Conversions|ToTransform(Vector) (Transformation|GetWorldLocation (Variables|Default|GetDefaultSceneRoot))) "Undefined" 0 0))
        (Utilities|Array|Add _mesharray_3 _returnvalue_3)))
    (:then_3
      (for _index_4 (range 0 (Variables|Default|GetNo%20of%20CoffCrunch))
        (bind _returnvalue_4 (Game|SpawnActorfromClass "/Game/Spirits_Calling/Blueprints/Trash/BP_CoffeeCrushed.BP_CoffeeCrushed_C" (Math|Conversions|ToTransform(Vector) (Transformation|GetWorldLocation (Variables|Default|GetDefaultSceneRoot))) "Undefined" 0 0))
        (Utilities|Array|Add _mesharray_3 _returnvalue_4)))
    (:then_4
      (for _index_5 (range 0 (Variables|Default|GetNo%20of%20Milk))
        (bind _returnvalue_5 (Game|SpawnActorfromClass "/Game/Spirits_Calling/Blueprints/Trash/BP_MilkCrushed.BP_MilkCrushed_C" (Math|Conversions|ToTransform(Vector) (Transformation|GetWorldLocation (Variables|Default|GetDefaultSceneRoot))) "Undefined" 0 0))
        (Utilities|Array|Add _mesharray _returnvalue_5)))
    (:then_5
      (for _index_6 (range 0 (Variables|Default|GetNo%20of%20Can))
        (bind _returnvalue_6 (Game|SpawnActorfromClass "/Game/Spirits_Calling/Blueprints/Trash/BP_CanCrunched.BP_CanCrunched_C" (Math|Conversions|ToTransform(Vector) (Transformation|GetWorldLocation (Variables|Default|GetDefaultSceneRoot))) "Undefined" 0 0))
        (Utilities|Array|Add _mesharray _returnvalue_6)))
    (:then_6
      (for _index_7 (range 0 (Variables|Default|GetNo%20of%20TBags))
        (bind _returnvalue_7 (Game|SpawnActorfromClass "/Game/Spirits_Calling/Blueprints/Trash/BP_TrashBags.BP_TrashBags_C" (Math|Conversions|ToTransform(Vector) (Transformation|GetWorldLocation (Variables|Default|GetDefaultSceneRoot))) "Undefined" 0 0))
        (Utilities|Array|Add _mesharray _returnvalue_7)))
    (:then_7
      ;[1 1 1] Create dissolve material instance
      (bind _returnvalue_8 (Rendering|Material|CreateDynamicMaterialInstance "/Game/Spirits_Calling/0_Testing_Alex/DissolveFX/FX2/M_Dissolve_2.M_Dissolve_2" "None" "None" :!class /Script/Engine.KismetMaterialLibrary))
      (Variables|Default|SetDissolveMaterial _returnvalue_8))))

(fn ConstructionScript
  (Variables|Default|SetNumberofMeshes (Math|Integer|Clamp(Integer) (Variables|Default|GetNumberofMeshes) 0 5))
  (for _index (range 0 (Variables|Default|GetNumberofMeshes))
    _))