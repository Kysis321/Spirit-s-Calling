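; Game mode for Spirits Calling that creates the HUD and handles player respawning.
; On BeginPlay it adds the HUD widget to the viewport and binds Respwan to the player character's OnDestroyed event.
; Respwan spawns a ThirdPersonCharacter at LastCheckpoint, or a ThirdPersonCharacter_Bec at the first PlayerStart when no checkpoint is valid.
; Each new character is possessed and rebound, so respawning repeats on every death.
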(event Custom|Respwan
  (params (DestroyedActor :type Actor%20Object%20Reference))
  (bind _lastcheckpoint (Variables|Default|GetLastCheckpoint))
  ;[1 1 1] Respawn mechanic
  (Utilities|IsValid _lastcheckpoint
    (:Is%20Valid
      (bind _returnvalue (Game|SpawnActorfromClass "/Game/DreamscapeSeries/SharedResources/Blueprints/ThirdPersonCharacter.ThirdPersonCharacter_C" (Math|Transform|MakeTransform (Transformation|GetActorLocation _lastcheckpoint) "0, 0, 0" "1,1,1") "Undefined" 0 0))
      (Game|BindEventtoOnDestroyed _returnvalue (delegate Custom|Respwan))
      (Pawn|Possess (Game|GetPlayerController 0) _returnvalue))
    (:Is%20Not%20Valid
      (bind _outactors (Actor|GetAllActorsOfClass "/Script/Engine.PlayerStart"))
      (bind _returnvalue_2 (Game|SpawnActorfromClass "/Game/Spirits_Calling/0_Testing_Bec/Blue_Prints/ThirdPersonCharacter_Bec.ThirdPersonCharacter_Bec_C" (Math|Transform|MakeTransform (Transformation|GetActorLocation (Utilities|Array|Get(acopy) _outactors)) "0, 0, 0" "1,1,1") "Undefined" 0 0))
      (Game|BindEventtoOnDestroyed _returnvalue_2 (delegate Custom|Respwan))
      (Pawn|Possess (Game|GetPlayerController 0) _returnvalue_2))))

(event EventBeginPlay
  ;[1 1 1] Setting up HUD
  (bind _returnvalue (UserInterface|CreateWidget "/Game/Spirits_Calling/Blueprints/UI_Blueprints/HeadsUpDisplay_UI.HeadsUpDisplay_UI_C"))
  (bind _output_get (Variables|Default|SetHeadsUpDisplay _returnvalue))
  (UserInterface|Viewport|AddtoViewport _output_get 0)
  ;[1 1 1] Respawn mechanic
  (Game|BindEventtoOnDestroyed (Game|GetPlayerCharacter 0) (delegate Custom|Respwan)))

(fn ConstructionScript)