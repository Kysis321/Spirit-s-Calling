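; Test shrine actor that the player activates once with Interact, notifying GM_SpiritsCalling that a shrine was collected and swapping to a triggered material.
; Trigger overlap by the ThirdPersonCharacter enables input and, while the shrine is still off, shows a prompt widget and opens a Gate for the interact event.
; Leaving disables input, removes the prompt and resets the DoOnce MultiInput, which closes the Gate.
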(event OnComponentBeginOverlap(ShrineTrigger)
  (params (OverlappedComponent :type Primitive%20Component%20Object%20Reference) (OtherActor :type Actor%20Object%20Reference) (OtherComp :type Primitive%20Component%20Object%20Reference) (OtherBodyIndex :type Integer) (bFromSweep :type Boolean) (SweepResult :type Hit%20Result%20Structure%20%28by%20ref%29))
  (bind _returnvalue (Game|GetPlayerController 0))
  (bind _asthird_person_character (Utilities|Casting|CastToThirdPersonCharacter OtherActor))
  (Input|EnableInput _returnvalue)
  (if (Variables|Default|GetIsShrineOff)
    (bind _returnvalue_2 (UserInterface|CreateWidget "/Game/Spirits_Calling/Blueprints/UI_Interact_Prompt_Widget.UI_Interact_Prompt_Widget_C" _returnvalue))
    (bind _output_get (Variables|Default|SetPromptWidget _returnvalue_2))
    (UserInterface|Viewport|AddtoViewport _output_get 0)
    (Variables|Default|SetPrompt (Variables|Default|GetPrompt))
    (|DoOnceMultiInput
      (:A%20Out
        (Default|ShowPrompt _asthird_person_character (Variables|Default|GetPrompt))
        (Utilities|FlowControl|Gate false) ; enters at Open
      )
      (:Reset%20Out
        (Development|PrintString "")
        (Utilities|FlowControl|Gate false) ; enters at Close
      ))))

(event OnComponentEndOverlap(ShrineTrigger)
  (params (OverlappedComponent :type Primitive%20Component%20Object%20Reference) (OtherActor :type Actor%20Object%20Reference) (OtherComp :type Primitive%20Component%20Object%20Reference) (OtherBodyIndex :type Integer))
  (bind _asthird_person_character (Utilities|Casting|CastToThirdPersonCharacter OtherActor))
  (Input|DisableInput (Game|GetPlayerController 0))
  (Widget|RemovefromParent (stale OnComponentBeginOverlap(ShrineTrigger) _output_get))
  (Default|HidePrompt _asthird_person_character)
  (|DoOnceMultiInput) ; enters at Reset In
)

(event Input|ActionEvents|InputActionInteract
  (params (Key :type Key%20Structure :default "None"))
  (:Pressed
    (Utilities|FlowControl|Gate false
      (:Exit
        (bind _asgm_spirits_calling (Utilities|Casting|CastToGM_SpiritsCalling (Game|GetGameMode)))
        (if (Variables|Default|GetIsShrineOff)
          (Default|CollectedShrines _asgm_spirits_calling)
          (Variables|Default|SetIsShrineOff false)
          (Rendering|Material|SetMaterial (Variables|Default|GetShrine) 0 (Variables|Default|GetTriggeredMaterial))
          (Development|PrintString "Input Disabled"))))))

(fn ConstructionScript)