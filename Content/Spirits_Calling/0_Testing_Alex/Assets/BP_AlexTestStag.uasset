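; Test stag actor that opens the skill purchase window when the player interacts with it.
; Overlapping StagTrigger enables input, shows a prompt and opens a gate for Interact; leaving reverses this through a DoOnce MultiInput reset.
; Interact plays the stag's voice, blends the view to the stag, hides the player, then shows UI_SkillWindow after a short delay and links it to the character and purchase buttons.
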(event OnComponentBeginOverlap(StagTrigger)
  (params (OverlappedComponent :type Primitive%20Component%20Object%20Reference) (OtherActor :type Actor%20Object%20Reference) (OtherComp :type Primitive%20Component%20Object%20Reference) (OtherBodyIndex :type Integer) (bFromSweep :type Boolean) (SweepResult :type Hit%20Result%20Structure%20%28by%20ref%29))
  (bind _returnvalue (Game|GetPlayerController 0))
  (bind _returnvalue_2 (Game|GetPlayerCharacter 0))
  ;[1 1 1] Enabling interaction with the E key when in the overlap (StagTrigger)
  (bind _asthird_person_character (Utilities|Casting|CastToThirdPersonCharacter OtherActor))
  (Input|EnableInput (Game|GetPlayerController 0))
  (bind _returnvalue_3 (UserInterface|CreateWidget "/Game/Spirits_Calling/Blueprints/UI_Blueprints/UI_Interact_Prompt_Widget.UI_Interact_Prompt_Widget_C"))
  (bind _output_get (Variables|Default|SetPromptWidget _returnvalue_3))
  (UserInterface|Viewport|AddtoViewport _output_get 0)
  (Variables|Default|SetPrompt (Variables|Default|GetPrompt))
  (|DoOnceMultiInput
    (:A%20Out
      (Default|ShowPrompt _asthird_person_character (Variables|Default|GetPrompt))
      (Utilities|FlowControl|Gate true) ; enters at Open
    )
    (:Reset%20Out
      (Development|PrintString "")
      (Utilities|FlowControl|Gate true) ; enters at Close
    )))

(event OnComponentEndOverlap(StagTrigger)
  (params (OverlappedComponent :type Primitive%20Component%20Object%20Reference) (OtherActor :type Actor%20Object%20Reference) (OtherComp :type Primitive%20Component%20Object%20Reference) (OtherBodyIndex :type Integer))
  (bind _returnvalue (Game|GetPlayerController 0))
  (bind _returnvalue_2 (Game|GetPlayerCharacter 0))
  ;[1 1 1] Enabling interaction with the E key when in the overlap (StagTrigger)
  (bind _asthird_person_character (Utilities|Casting|CastToThirdPersonCharacter OtherActor))
  (Input|DisableInput (Game|GetPlayerController 0))
  (Widget|RemovefromParent (stale OnComponentBeginOverlap(StagTrigger) _output_get))
  (Default|HidePrompt _asthird_person_character)
  (|DoOnceMultiInput) ; enters at Reset In
)

(event Input|ActionEvents|InputActionInteract
  (params (Key :type Key%20Structure))
  (bind _returnvalue (Game|GetPlayerController 0))
  (bind _returnvalue_2 (Game|GetPlayerCharacter 0))
  ;[1 1 1] Enabling interaction with the E key when in the overlap (StagTrigger)
  (:Pressed
    (if (not (Variables|Default|GetIsWindowOpen))
      (Utilities|FlowControl|Gate true
        (:Exit
          (bind _asthird_person_character (Utilities|Casting|CastToThirdPersonCharacter (Game|GetPlayerCharacter 0)))
          (Default|HidePrompt _asthird_person_character)
          ;[1 1 1] Changing camera, locking player character, hiding player character
          (Audio|PlaySoundatLocation "/Game/Spirits_Calling/Audio/NPC/Stag_Voice__audio_sample__Cue.Stag_Voice__audio_sample__Cue" (Transformation|GetActorLocation) "0, 0, 0" 1.0 1.0 0.0 0 0 0)
          (Game|Player|SetViewTargetwithBlend _returnvalue self 0.5 "VTBlend_Linear" 0.0 false)
          (bind _returnvalue_3 (UserInterface|CreateWidget "/Game/Spirits_Calling/Blueprints/UI_Blueprints/UI_SkillWindow.UI_SkillWindow_C" _returnvalue))
          (Variables|Default|SetSkillWindow _returnvalue_3)
          (Variables|/Script/Engine.PlayerController|SetbShowMouseCursor _returnvalue true)
          (Rendering|SetActorHiddenInGame _returnvalue_2 true)
          (Utilities|FlowControl|Delay 0.6)
          (UserInterface|Viewport|AddtoViewport (Variables|Default|GetSkillWindow) 0)
          (Input|SetInputModeGameandUI (Game|GetPlayerController 0) (Variables|Default|GetSkillWindow) "DoNotLock" false)
          (bind _asthird_person_character_2 (Utilities|Casting|CastToThirdPersonCharacter _returnvalue_2))
          (Variables|/Game/Spirits_Calling/Blueprints/ThirdPersonCharacter.ThirdPersonCharacter_C|SetIsSkillWindowOpen _asthird_person_character_2 true)
          (Variables|Default|SetIsWindowOpen true)
          (Variables|/Game/Spirits_Calling/Blueprints/ThirdPersonCharacter.ThirdPersonCharacter_C|SetSkillMenuUI _asthird_person_character_2 (Variables|Default|GetSkillWindow))
          (Variables|/Game/Spirits_Calling/Blueprints/UI_Blueprints/UI_SkillPurchaseButton.UI_SkillPurchaseButton_C|SetMySkillWindowUI (Variables|/Game/Spirits_Calling/Blueprints/UI_Blueprints/UI_SkillWindow.UI_SkillWindow_C|GetSkillPurchaseButton_DJ (Variables|Default|GetSkillWindow)) (Variables|Default|GetSkillWindow))
          (Variables|/Game/Spirits_Calling/Blueprints/UI_Blueprints/UI_SkillPurchaseButton.UI_SkillPurchaseButton_C|SetMySkillWindowUI (Variables|/Game/Spirits_Calling/Blueprints/UI_Blueprints/UI_SkillWindow.UI_SkillWindow_C|GetSkillPurchaseButton_D (Variables|Default|GetSkillWindow)) (Variables|Default|GetSkillWindow))
          (Variables|/Game/Spirits_Calling/Blueprints/UI_Blueprints/UI_SkillPurchaseButton.UI_SkillPurchaseButton_C|SetMySkillWindowUI (Variables|/Game/Spirits_Calling/Blueprints/UI_Blueprints/UI_SkillWindow.UI_SkillWindow_C|GetSkillPurchaseButton_GP (Variables|Default|GetSkillWindow)) (Variables|Default|GetSkillWindow)))))))

(fn ConstructionScript)