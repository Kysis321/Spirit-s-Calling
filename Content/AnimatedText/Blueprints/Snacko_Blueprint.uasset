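; Snacko actor Blueprint that puts a Text widget on screen when play begins, in the AnimatedText content.
; An unconnected, never-run section holds outdated speech bubble logic: it creates a SpeechbubbleOutdated widget and projects the Arrow component's world location to screen space.
; That section centers the bubble horizontally above the point, scaling its canvas slot size by viewport DPI scale.
; Tick and overlap events are empty.
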(event EventBeginPlay
  ;[1 1 1] whatever makes the bubble pop up (initialize dialogue)
  (bind _returnvalue (UserInterface|CreateWidget "/Game/AnimatedText/Blueprints/Text.Text_C"))
  (UserInterface|Viewport|AddtoViewport _returnvalue 0))

(event Collision|EventActorBeginOverlap
  (params (OtherActor :type Actor%20Object%20Reference)))

(event EventTick
  (params (DeltaSeconds :type Float%20%28single-precision%29))
  ;[1 1 1] for update of position
)

(fn ConstructionScript)